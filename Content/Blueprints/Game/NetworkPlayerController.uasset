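; Player controller for a networked game that spawns and possesses the player's pawn when play begins.
; On the local controller, BeginPlay reads the spectator flag from NetworkGameInstance, gets a spawn point from NetworkGameState and stores it as RespawnPoint.
; A server event then spawns either a SpectatorPawn or a NetworkPlayer at that point, always ignoring collisions, and possesses it.
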(event `self.ReceiveBeginPlay`
  ;[1 1 1] If this controller is local, spawn a pawn to possess in
  (if (`self.IsLocalPlayerController` self)
    (bind _asnetwork_game_instance (cast `/Game/Blueprints/NetworkGameInstance` (`GameplayStatics.GetGameInstance`))
      (:`then`
        (`self.PossessToSpawnablePawn` (`/Game/Blueprints/NetworkGameInstance.bIsSpectator` _asnetwork_game_instance)))
      (:`CastFailed`
        (`KismetSystemLibrary.PrintString` "Can`t do cast to networkGI")))))

(event `PossessToSpawnablePawn`
  (params (IsSpectatorMode :type Boolean))
  ;[1 1 1] Get spawnable point for adding pawn to it
  (bind _asnetwork_game_state (cast `/Game/Blueprints/Game/NetworkGameState` (`GameplayStatics.GetGameState`)))
  (bind _output (`/Game/Blueprints/Game/NetworkGameState.GetSpawnPoint` _asnetwork_game_state))
  (bind _output_get (set `self.RespawnPoint` _output))
  (`self.Server_SpawnPlayer` _output_get IsSpectatorMode))

(event `Server_SpawnPlayer`
  (params (SpawnPoint :type "Transform Structure") (IsSpectatorMode :type Boolean))
  ;[1 1 1] Spawn pawns only on the server
  (if IsSpectatorMode
    (bind _returnvalue (`|SpawnActorFromClass` "/Script/Engine.SpectatorPawn" SpawnPoint "AlwaysSpawn" "OverrideRootScale" null null))
    (`self.Possess` _returnvalue)
    (else
      (bind _returnvalue_2 (`|SpawnActorFromClass` "/Game/Blueprints/Game/NetworkPlayer.NetworkPlayer_C" SpawnPoint "AlwaysSpawn" "OverrideRootScale" null null))
      (`self.Possess` _returnvalue_2))))

(fn `UserConstructionScript`)